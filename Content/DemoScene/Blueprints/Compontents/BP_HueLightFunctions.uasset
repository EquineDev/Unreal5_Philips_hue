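; BP_HueLightFunctions links a physical Hue lamp to an in-game light source, dimming both as a tracked actor moves away.
; Setup functions store the lamp, light and location actors, and another copies the light's color to the lamp.
; When enabled, the update function scales both brightnesses by inverse distance, applying a multiplier and 0–254 clamp to the lamp.
; Its own event graph never runs the update.
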(fn `Configure Lights to Match`
  (params (LightSource :type "LightComponent Object Reference (by ref)"))
  (`HueLamp.SetColor` (`self.HueLamp`) (`KismetMathLibrary.Conv_LinearColorToColor` (`LightComponentBase.GetLightColor` LightSource))))

(fn `SetMultiplierHueLamp`
  (params (Amount :type Integer))
  (set `self.HueMultiplier ` Amount))

(fn `SetupActorRef`
  (params (ActorRef :type "Actor Object Reference (by ref)"))
  (set `self.ActorLocation` ActorRef))

(fn `SetupLightRef`
  (params (HueLampRef :type "HueLamp Object Reference (by ref)") (LightSourceRef :type "LightComponent Object Reference (by ref)") (LightActor :type "Actor Object Reference (by ref)"))
  (set `self.HueLamp` HueLampRef)
  (set `self.DigitalLightSource` LightSourceRef)
  (set `self.LightSourceLocation` LightActor))

(fn `UpdateLightSourceEvent`
  (params (Enable :type "Boolean (by ref)"))
  (bind _currentdistance (`self.Currentdistance`))
  (bind _returnvalue (`KismetMathLibrary.Vector_Distance` (`Actor.K2_GetActorLocation` (`self.ActorLocation`)) (`Actor.K2_GetActorLocation` (`self.LightSourceLocation`))))
  (if (and Enable (`KismetSystemLibrary.IsValid` (`self.HueLamp`)))
    (if (>= _returnvalue 1.0)
      (set `self.Currentdistance` (/ 1.0 _returnvalue))
      (`LightComponent.SetIntensity` (`self.DigitalLightSource`) (* (`self.DigitalBrightness`) _currentdistance))
      (`HueLamp.SetBrightness` (`self.HueLamp`) (`KismetMathLibrary.Clamp` (* (`KismetMathLibrary.FTrunc` (* _currentdistance (`self.HueBrightness`))) (`self.HueMultiplier `)) 0 254)))))