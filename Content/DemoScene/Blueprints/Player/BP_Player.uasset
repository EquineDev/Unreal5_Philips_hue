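; BP_Player is a demo first-person player with look and movement input and a weapon that works as a Hue light flare gun.
; On BeginPlay it casts the Weapon child actor to BP_Weapon and caches the reference, a simplified setup for demonstration.
; Fire passes the controller's view point to the weapon's FireGun, but only while InFiringRange, toggled through SetCanFire, is true.
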(event `self.ReceiveBeginPlay`
  ;[1 1 1] Weapon is more like set up like a singleton, its done for the sake simply showing how the hue lights can work as flare gun, rather than a production quality example
  (bind _asbp_weapon (cast `/HueLighting/DemoScene/Blueprints/Weapon/BP_Weapon` (`ChildActorComponent.ChildActor` (`self.Weapon`))))
  (set `self.WeaponRef` _asbp_weapon))

(event `/HueLighting/DemoScene/Blueprints/Player/BPI_PlayerInterface.LookYaw`
  (params (Axis :type "Float (double-precision)"))
  ;[1 1 1] Look
  (`self.AddControllerYawInput` Axis))

(event `/HueLighting/DemoScene/Blueprints/Player/BPI_PlayerInterface.LookPitch`
  (params (axis :type "Float (double-precision)"))
  ;[1 1 1] Look
  (`self.AddControllerPitchInput` (* -1.0 axis)))

(event `/HueLighting/DemoScene/Blueprints/Player/BPI_PlayerInterface.MoveForward`
  (params (Axis :type "Float (double-precision)"))
  ;[1 1 1] Movement
  (`self.AddMovementInput` (`self.GetActorForwardVector`) Axis))

(event `/HueLighting/DemoScene/Blueprints/Player/BPI_PlayerInterface.MoveRight`
  (params (Axis :type "Float (double-precision)"))
  ;[1 1 1] Movement
  (`self.AddMovementInput` (`self.GetActorRightVector`) Axis))

(event `/HueLighting/DemoScene/Blueprints/Player/BPI_PlayerInterface.Fire`
  (bind (_location _rotation) (`Controller.GetPlayerViewPoint` (`self.GetController`)))
  ;[1 1 1] Hue Light Lamp Projectile
  (if (and (`self.InFiringRange`) (`KismetSystemLibrary.IsValid` (`self.WeaponRef`)))
    (`/HueLighting/DemoScene/Blueprints/Weapon/BP_Weapon.FireGun` (`self.WeaponRef`) _location _rotation)))

(event `/HueLighting/DemoScene/Blueprints/Player/BPI_PlayerInterface.Set Can Fire`
  (params (Fire :type Boolean))
  ;[1 1 1] Hue Light Lamp Projectile
  (set `self.InFiringRange` Fire))

(fn `UserConstructionScript`)