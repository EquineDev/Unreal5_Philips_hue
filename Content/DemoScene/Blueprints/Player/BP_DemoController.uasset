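; BP_DemoController is the demo player controller that routes input to the controlled pawn and manages the WBP_HueMenu screen.
; On BeginPlay it caches the pawn through BPI_PlayerInterface and adds IMC_Default, then forwards Enhanced Input look and movement plus left-click fire as interface calls.
; SetupController creates and shows the menu, and Escape re-shows it, both pausing the game with UI-only input and a visible cursor.
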(event `self.ReceiveBeginPlay`
  (bind _returnvalue (pcsubsystem `EnhancedInputLocalPlayerSubsystem` self))
  ;[1 1 1] Get our interface of our player
  (bind _asbpi_player_interface (cast `/HueLighting/DemoScene/Blueprints/Player/BPI_PlayerInterface` (`self.K2_GetPawn`)))
  (set `self.PlayerPawn` _asbpi_player_interface)
  (`/Engine/EditorBlueprintResources/StandardMacros.IsValid` _returnvalue
    (:`Is Valid`
      (`EnhancedInputSubsystemInterface.AddMappingContext` _returnvalue "/HueLighting/DemoScene/Input/IMC_Default.IMC_Default" 0 (struct)))))

(event `Key|LeftMouseButton`
  (params (Key :type "Key Structure"))
  ;[1 1 1] Fire Player Weapon
  (:`Pressed`
    (`/HueLighting/DemoScene/Blueprints/Player/BPI_PlayerInterface.Fire` (`self.PlayerPawn`))))

(event `EnhancedInput|/HueLighting/DemoScene/Input/IA_Look`
  (params (ActionValue :type "Vector2D Structure") (ElapsedSeconds :type "Float (double-precision)") (TriggeredSeconds :type "Float (double-precision)") (InputAction :type "InputAction Object Reference" :default "/HueLighting/DemoScene/Input/IA_Look.IA_Look"))
  ;[1 1 1] Mouse Look
  (:`Triggered`
    (`/HueLighting/DemoScene/Blueprints/Player/BPI_PlayerInterface.LookYaw` (`self.PlayerPawn`) ActionValue_X)
    (`/HueLighting/DemoScene/Blueprints/Player/BPI_PlayerInterface.LookPitch` (`self.PlayerPawn`) ActionValue_Y)))

(event `EnhancedInput|/HueLighting/DemoScene/Input/IA_Movement`
  (params (ActionValue :type "Vector2D Structure") (ElapsedSeconds :type "Float (double-precision)") (TriggeredSeconds :type "Float (double-precision)") (InputAction :type "InputAction Object Reference" :default "/HueLighting/DemoScene/Input/IA_Movement.IA_Movement"))
  ;[1 1 1] Movement
  (:`Triggered`
    (`/HueLighting/DemoScene/Blueprints/Player/BPI_PlayerInterface.MoveRight` (`self.PlayerPawn`) ActionValue_X)
    (`/HueLighting/DemoScene/Blueprints/Player/BPI_PlayerInterface.MoveForward` (`self.PlayerPawn`) ActionValue_Y)))

(event `Key|Escape`
  (params (Key :type "Key Structure"))
  ;[1 1 1] Pause Game
  (:`Pressed`
    (if (not (`Widget.IsInViewport` (`self.HueUI`)))
      (`UserWidget.AddToViewport` (`self.HueUI`) 0)
      (`GameplayStatics.SetGamePaused` true)
      (`WidgetBlueprintLibrary.SetInputMode_UIOnlyEx` (`GameplayStatics.GetPlayerController` 0) (`self.HueUI`))
      (set `self.bShowMouseCursor` true))))

(fn `Setup Controller`
  ;[1 1 1] Get Refence to Player Pawn and Spawn Menu when player joins the game
  (bind _returnvalue (`|CreateWidget` "/HueLighting/DemoScene/UI/WBP_HueMenu.WBP_HueMenu_C"))
  (bind _output_get (set `self.HueUI` _returnvalue))
  (`UserWidget.AddToViewport` _output_get 0)
  (`GameplayStatics.SetGamePaused` true)
  (`KismetSystemLibrary.PrintString` "Post Login")
  (`WidgetBlueprintLibrary.SetInputMode_UIOnlyEx` (`GameplayStatics.GetPlayerController` 0) (`self.HueUI`))
  (set `self.bShowMouseCursor` true))

(fn `UserConstructionScript`)