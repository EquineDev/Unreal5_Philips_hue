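; BP_VirtualLamp is an in-level lamp that links its point light to a Hue lamp and responds to actors overlapping it.
; SetLamp binds the Hue lamp and passes both lights to BPDistanceCheck; unbound lamps print a warning on overlap.
; Overlap hands the actor to BPDistanceCheck and starts a looping timer driving its light-source updates.
; End overlap clears the timer and turns both lights off.
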(event `self.ReceiveActorBeginOverlap`
  (params (OtherActor :type "Actor Object Reference"))
  (if (`self.IsConfigured`)
    (set `self.CheckLightDistance` true)
    (`/HueLighting/DemoScene/Blueprints/Compontents/BP_HueLightFunctions.SetupActorRef` (`self.BP_DistanceCheck`) OtherActor)
    (`/HueLighting/DemoScene/Blueprints/Compontents/BP_HueLightFunctions.Configure Lights to Match` (`self.BP_DistanceCheck`) (`self.PointLight`))
    (bind _returnvalue (`KismetSystemLibrary.K2_SetTimerDelegate` (delegate `EventDisbatchForDistanceCheck`) 0.3 true))
    (set `self.LightBritness` _returnvalue)
    (else
      (`KismetSystemLibrary.PrintString` "Lamp Doesnt have refence to Lamp, Please BInd in Menu" true true (struct :`R` 1.0 :`B` 0.02448 :`A` 1.0)))))

(event `self.ReceiveActorEndOverlap`
  (params (OtherActor :type "Actor Object Reference"))
  (if (`self.IsConfigured`)
    (set `self.CheckLightDistance` false)
    (`KismetSystemLibrary.K2_ClearAndInvalidateTimerHandle` (`self.LightBritness`))
    (`self.TurnOffLights`)))

(event `EventDisbatchForDistanceCheck`
  (`/HueLighting/DemoScene/Blueprints/Compontents/BP_HueLightFunctions.UpdateLightSourceEvent` (`self.BP_DistanceCheck`) (`self.CheckLightDistance`)))

(fn `SetLamp`
  (params (SetLamp :type "HueLamp Object Reference"))
  (bind _pointlight (`self.PointLight`))
  (set `self.HueLightLamp` SetLamp)
  (set `self.IsConfigured` true)
  (`/HueLighting/DemoScene/Blueprints/Compontents/BP_HueLightFunctions.SetupLightRef` (`self.BP_DistanceCheck`) (`self.HueLightLamp`) _pointlight (`ActorComponent.GetOwner` _pointlight)))

(fn `TurnOffLights`
  (`/Engine/EditorBlueprintResources/StandardMacros.IsValid` (`self.HueLightLamp`)
    (:`Is Valid`
      (`LightComponent.SetIntensity` (`self.PointLight`) 0.0)
      (`HueLamp.SetBrightness` (`self.HueLightLamp`) 0))))

(fn `UserConstructionScript`)