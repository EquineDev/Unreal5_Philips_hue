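; BP_Weapon is a flare gun that fires lamp projectiles linked to a Hue lamp.
; SetupGun stores the lamp reference and arms the gun; FireGun then spawns a BP_ProjectileLamp, hands it the parent actor and lamp, and blocks further shots.
; It binds to the projectile's destroyed event, and CanReFire sets lamp brightness to zero and re-enables firing.
; Firing without a valid lamp prints an error.
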(fn `CanReFire`
  ;[1 1 1] Enable Refire and set hue lamp brightness to 0
  (`HueLamp.SetBrightness` (`self.LampRef`) 0)
  (set `self.CanFire` true))

(fn `FireGun`
  (params (Location :type "Vector Structure (by ref)") (Rotatation :type "Rotator Structure (by ref)"))
  ;[1 1 1] Fire Flare Gun
  (`/Engine/EditorBlueprintResources/StandardMacros.IsValid` (`self.LampRef`) ; Make Sure lamp if Valid
    (:`Is Valid`
      (if (`self.CanFIre`)
        (bind _returnvalue (`|SpawnActorFromClass` "/HueLighting/DemoScene/Blueprints/Weapon/BP_ProjectileLamp.BP_ProjectileLamp_C" (`KismetMathLibrary.MakeTransform` Location Rotatation) "Undefined" "OverrideRootScale" null null))
        (`/Engine/EditorBlueprintResources/StandardMacros.IsValid` _returnvalue
          (:`Is Valid`
            (`/HueLighting/DemoScene/Blueprints/Weapon/BP_ProjectileLamp.Setup` _returnvalue (`self.GetParentActor` self) (`self.LampRef`))
            (set `self.CanFIre` false)
            (add `/HueLighting/DemoScene/Blueprints/Weapon/BP_ProjectileLamp.OnLampProjectileDestroyed` _returnvalue (`|CreateDelegate` :!event `CanReFire`))))))
    (:`Is Not Valid`
      (`KismetSystemLibrary.PrintString` "Weapon Doesnt have refence to Lamp, Please BInd in Menu " true true (struct :`R` 1.0 :`B` 0.02448 :`A` 1.0)))))

(fn `SetupGun`
  (params (Lamp :type "HueLamp Object Reference"))
  ;[1 1 1] Setup our refrence to our Flare gun
  (set `self.LampRef` Lamp)
  (set `self.CanFire` true))

(fn `UserConstructionScript`)