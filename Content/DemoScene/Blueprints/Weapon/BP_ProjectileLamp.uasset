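; Lamp projectile weapon actor that carries a point light and links it to a Hue lamp through the BPDistanceCheck component.
; Setup gives the component the owner, lamp and light, then FireWeapon configures the lights to match, sets projectile speed and starts a looping timer.
; UpdateLightSources forwards light updates to the component.
; After TimeToLive the projectile calls its destroyed notification, clears the timer and destroys itself.
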(event `self.ReceiveBeginPlay`
  (`KismetSystemLibrary.Delay` (`self.TimeToLive`))
  (`self.OnLampProjectileDestroyed`)
  (`KismetSystemLibrary.K2_ClearAndInvalidateTimerHandle` (`self.LightTimer`))
  (`self.K2_DestroyActor`))

(fn `FireWeapon`
  (`/HueLighting/DemoScene/Blueprints/Compontents/BP_HueLightFunctions.Configure Lights to Match` (`self.BP_DistanceCheck`) (`self.PointLight`))
  (set `ProjectileMovementComponent.InitialSpeed` 1000.0 (`self.ProjectileMovement`))
  (bind _returnvalue (`KismetSystemLibrary.K2_SetTimerDelegate` (`|CreateDelegate` :!event `UpdateLightSources`) 0.1 true))
  (set `self.LightTimer` _returnvalue))

(fn `Setup`
  (params (Owner :type "Actor Object Reference (by ref)") (Lamp :type "HueLamp Object Reference (by ref)"))
  (bind _pointlight (`self.PointLight`))
  (`/HueLighting/DemoScene/Blueprints/Compontents/BP_HueLightFunctions.SetupActorRef` (`self.BP_DistanceCheck`) Owner)
  (`/HueLighting/DemoScene/Blueprints/Compontents/BP_HueLightFunctions.SetupLightRef` (`self.BP_DistanceCheck`) Lamp _pointlight (`ActorComponent.GetOwner` _pointlight))
  (`/HueLighting/DemoScene/Blueprints/Compontents/BP_HueLightFunctions.SetMultiplierHueLamp` (`self.BP_DistanceCheck`) 10)
  (`self.FireWeapon`))

(fn `UpdateLightSources`
  (`/HueLighting/DemoScene/Blueprints/Compontents/BP_HueLightFunctions.UpdateLightSourceEvent` (`self.BP_DistanceCheck`) (`KismetSystemLibrary.IsValid` self)))

(fn `UserConstructionScript`)